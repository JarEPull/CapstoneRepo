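; GenerateRooms assigns special types to the level's RoomGenerator actors, creating treasure rooms and one shop.
; Generate randomly retries until two treasures and one shop land on distinct rooms, calling ShowType on each.
; It excludes RoomGenerator9 by hardcoded object name, then gives that room its own fixed type.
; Nothing here calls Generate, and the event graph holds an unconnected earlier variant without that exclusion.
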(event EventBeginPlay)

(event Collision|EventActorBeginOverlap
  (params (OtherActor :type Actor%20Object%20Reference)))

(event EventTick
  (params (DeltaSeconds :type Float%20%28single-precision%29)))

(fn ConstructionScript)

(fn Generate
  (bind _outactors (Actor|GetAllActorsOfClass "/Game/Blueprints/RoomGenerator.RoomGenerator_C"))
  (while (< (Variables|Default|GettreasuresGenerated) 2)
    (bind _output_get (Variables|Default|SetroomSelected (.OutItem (Utilities|Array|Random _outactors))))
    (if (!= (Variables|/Game/Blueprints/RoomGenerator.RoomGenerator_C|GetroomType _output_get) 2)
      (if (Utilities|Enum|NotEqual(Enum) (Utilities|GetObjectName _output_get) "RoomGenerator9")
        (Variables|/Game/Blueprints/RoomGenerator.RoomGenerator_C|SetroomType _output_get 2)
        (Math|Integer|IncrementInt (Variables|Default|GettreasuresGenerated)
          (:%20%20
            (Default|ShowType _output_get))))))
  (while (not (Variables|Default|GetshopGenerated))
    (bind _output_get_2 (Variables|Default|SetroomSelected (.OutItem (Utilities|Array|Random _outactors))))
    (if (!= (Variables|/Game/Blueprints/RoomGenerator.RoomGenerator_C|GetroomType _output_get_2) 2)
      (if (!= (Variables|/Game/Blueprints/RoomGenerator.RoomGenerator_C|GetroomType _output_get_2) 1)
        (if (Utilities|Enum|NotEqual(Enum) (Utilities|GetObjectName _output_get_2) "RoomGenerator9")
          (Variables|/Game/Blueprints/RoomGenerator.RoomGenerator_C|SetroomType _output_get_2 1)
          (Variables|Default|SetshopGenerated true)
          (Default|ShowType _output_get_2)))))
  (bind _outactors_2 (Actor|GetAllActorsOfClass "/Game/Blueprints/RoomGenerator.RoomGenerator_C"))
  (bind _array_element (Utilities|Array|ForEachLoopwithBreak _outactors_2 :!label _label)
    (:LoopBody
      (if (Utilities|Enum|Equal(Enum) (Utilities|GetObjectName _array_element) "RoomGenerator9")
        (Variables|/Game/Blueprints/RoomGenerator.RoomGenerator_C|SetroomType _array_element 3)
        (Default|ShowType _array_element)
        (goto _label Break)))))