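; EvilGuy is an enemy spawner actor that picks a random enemy type on BeginPlay and brings it into play.
; It rolls a small chance for each EnemyTypes entry in the PlayerData game instance, rerunning the loop until one is chosen.
; It then shows a FightWidget for that enemy, spawns an EnemyPawn at its location, passes the type to the EnemyController and destroys itself.
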(event EventBeginPlay
  (bind _asplayer_data (Utilities|Casting|CastToPlayerData (Game|GetGameInstance)))
  (bind _array_element (Utilities|Array|ForEachLoopwithBreak (Variables|/Game/Blueprints/PlayerData.PlayerData_C|GetEnemyTypes _asplayer_data) :!label _label)
    (:LoopBody
      (if (not (Variables|Default|GethasEnemy))
        (if (== (Math|Random|RandomIntegerinRange 0 10) 1)
          (Variables|Default|SetEnemyRef _array_element)
          (Variables|Default|SethasEnemy true)
          (goto _label Break))))
    (:Completed
      (if (Variables|Default|GethasEnemy)
        (bind _returnvalue (UserInterface|CreateWidget "/Game/Widget/FightWidget.FightWidget_C"))
        (Variables|/Game/Widget/FightWidget.FightWidget_C|SetenemyReference _returnvalue (Variables|Default|GetEnemyRef))
        (UserInterface|Viewport|AddtoViewport _returnvalue 0)
        (bind _returnvalue_2 (Game|SpawnActorfromClass "/Game/Blueprints/EnemyPawn.EnemyPawn_C" (Math|Transform|MakeTransform (Transformation|GetWorldLocation (Variables|Default|GetDefaultSceneRoot)) "0, 0, 0" "1,1,1") "AlwaysSpawn" 0 0))
        (bind _asenemy_controller (Utilities|Casting|CastToEnemyController (AI|GetAIController _returnvalue_2))
          (:then
            (Variables|/Game/Blueprints/EnemyController.EnemyController_C|SetEnemyRef _asenemy_controller (Variables|Default|GetEnemyRef))
            (Actor|DestroyActor))
          (:CastFailed
            (Development|PrintString "controller cast failed")))
        (else
          (goto _label))))))

(event Collision|EventActorBeginOverlap
  (params (OtherActor :type Actor%20Object%20Reference)))

(event EventTick
  (params (DeltaSeconds :type Float%20%28single-precision%29)))

(fn ConstructionScript)