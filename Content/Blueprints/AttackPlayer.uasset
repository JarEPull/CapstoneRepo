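; AttackPlayer is a Behavior Tree task that runs an enemy's attack in turn-based combat.
; It finds top-level FightWidget instances and calls EnemyAttack on them, so the attack itself is delegated to the UI widget.
; A one-second Delay loop polls the widget's EnemyDoneAttacking flag.
; Once that is set, the task clears IsTurn on the EnemyController, resets its local flag and finishes successfully.
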(event EventReceiveExecuteAI
  (params (OwnerController :type AI%20Controller%20Object%20Reference) (ControlledPawn :type Pawn%20Object%20Reference))
  (bind _foundwidgets (Widget|GetAllWidgetsOfClass "/Game/Widget/FightWidget.FightWidget_C" true))
  (for _array_element _foundwidgets
    (bind _asfight_widget (Utilities|Casting|CastToFightWidget _array_element)
      (:then
        (Default|EnemyAttack _asfight_widget))
      (:CastFailed
        (Development|PrintString "FailedCast"))))
  (if (Variables|Default|GetdoneAttacking) :!label _label
    (bind _asenemy_controller (Utilities|Casting|CastToEnemyController OwnerController)
      (:then
        (Variables|/Game/Blueprints/EnemyController.EnemyController_C|SetisTurn _asenemy_controller false)
        (Variables|Default|SetdoneAttacking false)
        (AI|BehaviorTree|FinishExecute true))
      (:CastFailed
        (Development|PrintString "Wrong Controller")))
    (else
      (Utilities|FlowControl|Delay 1.0)
      (Variables|Default|SetdoneAttacking (Variables|/Game/Widget/FightWidget.FightWidget_C|GetenemyDoneAttacking _asfight_widget))
      (goto _label))))