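; Player pawn for the tower that advances between numbered MovementPoint actors and handles the pause menu.
; MoveToNextPoint finds the next point by index, starts the movement timeline and tells the Adventurer to move.
; The timeline lerps the pawn's location, then asks TowerPController to generate a room when finished.
; The Pause input toggles PauseWidget, freezing play through zero global time dilation rather than engine pause.
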(event Custom|Movement
  (bind _movetrack (Timeline|MovementTimeline PlayFromStart)
    (:Update
      (Transformation|SetActorLocation (Math|Vector|Lerp(Vector) (Variables|Default|GetcurrPointLoc) (Variables|Default|GetnextPointLoc) _movetrack) false false))
    (:Finished
      (bind _astower_pcontroller (Utilities|Casting|CastToTowerPController (Game|GetPlayerController 0)))
      (Default|GenerateRoom _astower_pcontroller))))

(event EventBeginPlay
  (Input|SetInputModeGameandUI (Game|GetPlayerController 0) 0 "DoNotLock" true))

(event Collision|EventActorBeginOverlap
  (params (OtherActor :type Actor%20Object%20Reference)))

(event EventTick
  (params (DeltaSeconds :type Float%20%28single-precision%29)))

(event Input|ActionEvents|InputActionPause
  (params (Key :type Key%20Structure :default "None"))
  (:Pressed
    (bind _output_get (Variables|Default|SetwidgetCount 0))
    (bind _foundwidgets (Widget|GetAllWidgetsOfClass "/Game/Widget/PauseWidget.PauseWidget_C" true))
    (for _array_element _foundwidgets
      (Math|Integer|IncrementInt _output_get))
    (if (!= (Variables|Default|GetwidgetCount) 0)
      (Utilities|Time|SetGlobalTimeDilation 1.0)
      (bind _foundwidgets_2 (Widget|GetAllWidgetsOfClass "/Game/Widget/PauseWidget.PauseWidget_C" true))
      (for _array_element_2 _foundwidgets_2
        (Widget|RemovefromParent _array_element_2))
      (else
        (bind _returnvalue (UserInterface|CreateWidget "/Game/Widget/PauseWidget.PauseWidget_C"))
        (UserInterface|Viewport|AddtoViewport _returnvalue 99)
        (Utilities|Time|SetGlobalTimeDilation 0.0)))))

(fn ConstructionScript)

(fn MovetoNextPoint
  (bind _outactors (Actor|GetAllActorsOfClass "/Game/Blueprints/MovementPoint.MovementPoint_C"))
  (bind _array_element (Utilities|Array|ForEachLoopwithBreak _outactors)
    (:LoopBody
      (if (== (Variables|/Game/Blueprints/MovementPoint.MovementPoint_C|Getlocation _array_element) (Variables|Default|GetcurrPoint))
        (Variables|Default|SetcurrPointLoc (Transformation|GetWorldLocation (Variables|/Game/Blueprints/MovementPoint.MovementPoint_C|GetDefaultSceneRoot _array_element)))
        (elif (not (Variables|Default|GetcurrPointCompleted))
          (if (== (Variables|/Game/Blueprints/MovementPoint.MovementPoint_C|Getlocation _array_element) (+ (Variables|Default|GetcurrPoint) 1))
            (Variables|Default|SetcurrPointCompleted true)
            (Variables|Default|SetcurrPoint (+ (Variables|Default|GetcurrPoint) 1))
            (Variables|Default|SetnextPointLoc (Transformation|GetWorldLocation (Variables|/Game/Blueprints/MovementPoint.MovementPoint_C|GetDefaultSceneRoot _array_element)))
            (CallFunction|Movement)
            (bind _returnvalue (Actor|GetActorOfClass "/Game/Blueprints/Adventurer.Adventurer_C"))
            (Default|MovePoints _returnvalue)))))
    (:Completed
      (Variables|Default|SetcurrPointCompleted false))))