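; Adventurer actor that moves through the level one numbered AdventurerMovePoint at a time.
; MovePoints scans all move point actors, caches the location matching CurrPoint, then advances to the next index and stores its location.
; A guard flag limits this to one step per call, which fires the Movement event.
; Movement plays a timeline that lerps the actor between the two stored locations without sweep.
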(event Custom|Movement
  (bind _movetrack (Timeline|AdventurerTimeline PlayFromStart)
    (:Update
      (Transformation|SetActorLocation (Math|Vector|Lerp(Vector) (Variables|Default|GetcurrPointLoc) (Variables|Default|GetnextPointLoc) _movetrack) false false))))

(event EventBeginPlay)

(event Collision|EventActorBeginOverlap
  (params (OtherActor :type Actor%20Object%20Reference)))

(event EventTick
  (params (DeltaSeconds :type Float%20%28single-precision%29)))

(fn ConstructionScript)

(fn MovePoints
  (bind _outactors (Actor|GetAllActorsOfClass "/Game/Blueprints/AdventurerMovePoint.AdventurerMovePoint_C"))
  (bind _array_element (Utilities|Array|ForEachLoopwithBreak _outactors)
    (:LoopBody
      (if (== (Variables|/Game/Blueprints/AdventurerMovePoint.AdventurerMovePoint_C|GetPointLoc _array_element) (Variables|Default|GetcurrPoint))
        (Variables|Default|SetcurrPointLoc (Transformation|GetWorldLocation (Variables|/Game/Blueprints/AdventurerMovePoint.AdventurerMovePoint_C|GetDefaultSceneRoot _array_element)))
        (elif (not (Variables|Default|GetcurrPointCompleted))
          (if (== (Variables|/Game/Blueprints/AdventurerMovePoint.AdventurerMovePoint_C|GetPointLoc _array_element) (+ (Variables|Default|GetcurrPoint) 1))
            (Variables|Default|SetcurrPointCompleted true)
            (Variables|Default|SetcurrPoint (+ (Variables|Default|GetcurrPoint) 1))
            (Variables|Default|SetnextPointLoc (Transformation|GetWorldLocation (Variables|/Game/Blueprints/AdventurerMovePoint.AdventurerMovePoint_C|GetDefaultSceneRoot _array_element)))
            (CallFunction|Movement)))))
    (:Completed
      (Variables|Default|SetcurrPointCompleted false))))