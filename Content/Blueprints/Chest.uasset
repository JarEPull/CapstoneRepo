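; Chest Blueprint that generates a random weapon as loot for a chest widget or the Shopkeep.
; Unless flagged as a shopkeep chest, BeginPlay rolls a weighted rarity and sets a level multiplier from the map name.
; LootGeneration randomly picks from PlayerData's weapon variations, repeating the pass until one hits, then scales damage by rarity and level.
; The caller name decides whether the weapon opens a ChestWidget or goes to the Shopkeep.
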(event EventBeginPlay
  (if (not (Variables|Default|GetShopkeepChest))
    (bind _output_get (Variables|Default|SetRollLoot (Math|Random|RandomIntegerinRange 1 100)))
    (if (>= _output_get 50)
      (if (>= _output_get 75)
        (if (>= _output_get 90)
          (if (>= _output_get 97)
            (Variables|Default|SetRarity 4)
            (else
              (Variables|Default|SetRarity 3)))
          (else
            (Variables|Default|SetRarity 2)))
        (else
          (Variables|Default|SetRarity 1)))
      (else
        (Variables|Default|SetRarity 0)))
    (bind _returnvalue (Game|GetCurrentLevelName true))
    (if (Utilities|Enum|Equal(Enum) _returnvalue "TutorialWorld")
      (Variables|Default|SetLevelMult 0.5)
      (Variables|Default|SetWeapLevel "T")
      (elif (Utilities|Enum|Equal(Enum) _returnvalue "World1")
        (Variables|Default|SetLevelMult 1.0)
        (Variables|Default|SetWeapLevel "1")
        (elif (Utilities|Enum|Equal(Enum) _returnvalue "World2")
          (Variables|Default|SetLevelMult 1.5)
          (Variables|Default|SetWeapLevel "2")
          (else
            (Variables|Default|SetLevelMult 2.0)
            (Variables|Default|SetWeapLevel "3")))))
    (CallFunction|LootGeneration "Chest")))

(event Collision|EventActorBeginOverlap
  (params (OtherActor :type Actor%20Object%20Reference)))

(event EventTick
  (params (DeltaSeconds :type Float%20%28single-precision%29)))

(fn ConstructionScript)

(fn LootGeneration
  (params (WhoCalled :type String))
  (bind _levelmult (Variables|Default|GetLevelMult))
  (Variables|Default|SetWhoCalled WhoCalled)
  (switch int (Variables|Default|GetRarity)
    (:0
      (Variables|Default|SetRarityName "Common")
      (Variables|Default|SetDamageMult 1.0)
      (Variables|Default|SetRarityColor "(R=0.721875,G=0.721875,B=0.721875,A=1.000000)"))
    (:1
      (Variables|Default|SetRarityName "Uncommon")
      (Variables|Default|SetDamageMult 1.25)
      (Variables|Default|SetRarityColor "(R=0.018128,G=0.666667,B=0.011111,A=1.000000)"))
    (:2
      (Variables|Default|SetRarityName "Rare")
      (Variables|Default|SetDamageMult 1.5)
      (Variables|Default|SetRarityColor "(R=0.000000,G=0.078362,B=1.000000,A=1.000000)"))
    (:3
      (Variables|Default|SetRarityName "Epic")
      (Variables|Default|SetDamageMult 1.75)
      (Variables|Default|SetRarityColor "(R=0.416059,G=0.000000,B=1.000000,A=1.000000)"))
    (:4
      (Variables|Default|SetRarityName "Legendary")
      (Variables|Default|SetDamageMult 2.0)
      (Variables|Default|SetRarityColor "(R=1.000000,G=0.325192,B=0.000000,A=1.000000)")))
  (bind _asplayer_data (Utilities|Casting|CastToPlayerData (Game|GetGameInstance)))
  (bind _array_element (Utilities|Array|ForEachLoopwithBreak (Variables|/Game/Blueprints/PlayerData.PlayerData_C|GetWeaponVariations _asplayer_data) :!label _label)
    (:LoopBody
      (bind _output_get (Variables|Default|SetRollLoot (Math|Random|RandomIntegerinRange 1 10)))
      (if (== _output_get 1)
        (if (Variables|Default|GetWeaponAlreadyGenerated)
          (goto _label Break)
          (else
            (Variables|Default|SetWeaponGenerated _array_element)
            (Variables|Default|SetWeaponAlreadyGenerated true)))))
    (:Completed
      (if (Variables|Default|GetWeaponAlreadyGenerated)
        (Variables|Default|SetWeapon (Utilities|Struct|MakeWeapon (.weaponname (Variables|Default|GetWeaponGenerated)) (Math|Float|Round (* (* (.damagemin (Variables|Default|GetWeaponGenerated)) (Variables|Default|GetDamageMult)) _levelmult)) (Math|Float|Round (* (* (.damagemax (Variables|Default|GetWeaponGenerated)) (Variables|Default|GetDamageMult)) _levelmult)) (.dicemax (Variables|Default|GetWeaponGenerated)) (.bonustohit (Variables|Default|GetWeaponGenerated)) (Variables|Default|GetRarityName) (Variables|Default|GetRarityColor) (Variables|Default|GetWeapLevel)))
        (switch string (Variables|Default|GetWhoCalled)
          (:Chest
            (CallFunction|CreateChestWidget))
          (:Shop
            (bind _returnvalue (Actor|GetActorOfClass "/Game/Blueprints/Shopkeep.Shopkeep_C"))
            (Default|ReceiveWeapon _returnvalue (Variables|Default|GetWeapon))))
        (else
          (goto _label))))))

(fn CreateChestWidget
  (bind _returnvalue (UserInterface|CreateWidget "/Game/Widget/ChestWidget.ChestWidget_C" 0 (Variables|Default|GetWeapon)))
  (UserInterface|Viewport|AddtoViewport _returnvalue 0))