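; Room actor that colors its cube by room type and helps start room generation at BeginPlay.
; In TutorialWorld, each instance maps its RoomNum to a fixed RoomType, then ShowType applies the matching material.
; In other levels it shows its existing type, and only the instance named RoomGenerator1 then calls Generate on the GenerateRooms actor, using the object name as a run-once gate.
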(event EventBeginPlay
  (bind _returnvalue (Game|GetCurrentLevelName true))
  (if (Utilities|Enum|Equal(Enum) _returnvalue "TutorialWorld")
    (switch int (Variables|Default|GetroomNum)
      (:0
        (Variables|Default|SetroomType 4))
      (:1
        (Variables|Default|SetroomType 0))
      (:2
        (Variables|Default|SetroomType 2))
      (:3
        (Variables|Default|SetroomType 0))
      (:4
        (Variables|Default|SetroomType 1))
      (:5
        (Variables|Default|SetroomType 3)))
    (CallFunction|ShowType)
    (else
      (CallFunction|ShowType)
      (if (Utilities|Enum|Equal(Enum) (Utilities|GetObjectName self) "RoomGenerator1")
        (bind _returnvalue_2 (Actor|GetActorOfClass "/Game/Blueprints/GenerateRooms.GenerateRooms_C"))
        (Default|Generate _returnvalue_2)))))

(event Collision|EventActorBeginOverlap
  (params (OtherActor :type Actor%20Object%20Reference)))

(event EventTick
  (params (DeltaSeconds :type Float%20%28single-precision%29)))

(fn ConstructionScript)

(fn ShowType
  (bind _cube (Variables|Default|GetCube))
  (switch int (Variables|Default|GetroomType)
    (:0
      (Rendering|Material|SetMaterial _cube 0 "/Game/Material/Red.Red"))
    (:1
      (Rendering|Material|SetMaterial _cube 0 "/Game/Material/Blue.Blue"))
    (:2
      (Rendering|Material|SetMaterial _cube 0 "/Game/Material/Yellow.Yellow"))
    (:3
      (Rendering|Material|SetMaterial _cube 0 "/Game/Material/Purple.Purple"))
    (:4
      (Rendering|Material|SetMaterial _cube 0 "/Game/Material/DarkGrey.DarkGrey"))))