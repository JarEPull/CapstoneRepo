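; Tower controller that populates the player's current room with its encounter when play begins.
; GenerateRoom finds the RoomGenerator whose RoomNum matches the TowerPawn's CurrPoint and reads its room type and cube location.
; The type selects an enemy, shopkeeper, chest or old man to spawn at a fixed offset from the cube; type 3 spawns nothing.
; The old man's room also opens a textbox widget with placeholder tutorial text.
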(event EventBeginPlay
  (CallFunction|GenerateRoom))

(event EventTick
  (params (DeltaSeconds :type Float%20%28single-precision%29)))

(fn ConstructionScript)

(fn GenerateRoom
  (bind _astower_pawn (Utilities|Casting|CastToTowerPawn (Game|Player|GetPlayerPawn 0)))
  (bind _outactors (Actor|GetAllActorsOfClass "/Game/Blueprints/RoomGenerator.RoomGenerator_C"))
  (bind _array_element (Utilities|Array|ForEachLoopwithBreak _outactors :!label _label)
    (:LoopBody
      (if (== (Variables|/Game/Blueprints/RoomGenerator.RoomGenerator_C|GetroomNum _array_element) (Variables|/Game/Blueprints/TowerPawn.TowerPawn_C|GetcurrPoint _astower_pawn))
        (Variables|Default|SettypeToGenerate (Variables|/Game/Blueprints/RoomGenerator.RoomGenerator_C|GetroomType _array_element))
        (Variables|Default|SetroomLoc (Transformation|GetWorldLocation (Variables|/Game/Blueprints/RoomGenerator.RoomGenerator_C|GetCube _array_element)))
        (goto _label Break)))
    (:Completed
      (switch int (Variables|Default|GettypeToGenerate)
        (:0
          (Game|SpawnActorfromClass "/Game/Blueprints/EvilGuy.EvilGuy_C" (Math|Transform|MakeTransform (Math|Vector|MakeVector (.x (Variables|Default|GetroomLoc)) (+ (.y (Variables|Default|GetroomLoc)) 3e+02) (+ (.z (Variables|Default|GetroomLoc)) 8e+01)) "0, 0, 0" "1,1,1") "Undefined" 0 0))
        (:1
          (Game|SpawnActorfromClass "/Game/Blueprints/Shopkeep.Shopkeep_C" (Math|Transform|MakeTransform (Math|Vector|MakeVector (.x (Variables|Default|GetroomLoc)) (+ (.y (Variables|Default|GetroomLoc)) 3e+02) (+ (.z (Variables|Default|GetroomLoc)) 8e+01)) "0, 0, 0" "1,1,1") "Undefined" 0 0))
        (:2
          (Game|SpawnActorfromClass "/Game/Blueprints/Chest.Chest_C" (Math|Transform|MakeTransform (Math|Vector|MakeVector (.x (Variables|Default|GetroomLoc)) (+ (.y (Variables|Default|GetroomLoc)) 3e+02) (+ (.z (Variables|Default|GetroomLoc)) 8e+01)) "0, 0, 0" "1,1,1") "Undefined" 0 false 0))
        (:4
          (Game|SpawnActorfromClass "/Game/Blueprints/OldMan.OldMan_C" (Math|Transform|MakeTransform (Math|Vector|MakeVector (.x (Variables|Default|GetroomLoc)) (+ (.y (Variables|Default|GetroomLoc)) 3e+02) (+ (.z (Variables|Default|GetroomLoc)) 8e+01)) "0, 0, 0" "1,1,1") "Undefined" 0 0)
          (bind _returnvalue (UserInterface|CreateWidget "/Game/Widget/TextboxWidget.TextboxWidget_C" 0 "Tutorial text goes here. Attack for damage, abilities do stuff, blah blah lorem ipsum." "Old Man"))
          (UserInterface|Viewport|AddtoViewport _returnvalue 0))))))